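; Pickup spawn point that spawns a configurable actor on BeginPlay and respawns it after a delay once that actor is destroyed.
; Its collision sphere shows a text prompt on overlap and adds or removes the actor in Character_RobHat's pickup list.
; The spawned actor is set to replicate and receives the spawner via BindBePickUpMessage, a coupling the comments flag.
; A RepNotify on IsOpenCollision mirrors the sphere's collision toggle to clients.
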(event OnComponentBeginOverlap(CollisionSphere)
  (params (OverlappedComponent :type Primitive%20Component%20Object%20Reference) (OtherActor :type Actor%20Object%20Reference) (OtherComp :type Primitive%20Component%20Object%20Reference) (OtherBodyIndex :type Integer) (bFromSweep :type Boolean) (SweepResult :type Hit%20Result%20Structure%20%28by%20ref%29))
  ;[1 1 1] 维护Pawn的可拾取物品List
  (bind _ascharacter_rob_hat (Utilities|Casting|CastToCharacter_RobHat OtherActor))
  (Rendering|SetVisibility (Variables|Default|GetTextRender) true false)
  (Default|EventAddtoPickUpList _ascharacter_rob_hat (Variables|Default|GetActorToSpawn)))

(event OnComponentEndOverlap(CollisionSphere)
  (params (OverlappedComponent :type Primitive%20Component%20Object%20Reference) (OtherActor :type Actor%20Object%20Reference) (OtherComp :type Primitive%20Component%20Object%20Reference) (OtherBodyIndex :type Integer))
  ;[1 1 1] 维护Pawn的可拾取物品List
  (Rendering|SetVisibility (Variables|Default|GetTextRender) false false)
  (bind _ascharacter_rob_hat (Utilities|Casting|CastToCharacter_RobHat OtherActor))
  (Default|EventRemovetoPickUpList _ascharacter_rob_hat (Variables|Default|GetActorToSpawn)))

(event Custom|Event_OnActorDestroyed
  (params (DestroyedActor :type Actor%20Object%20Reference))
  ;[1 1 1] 生成Actor并配置自动生成和特殊配置
  (Utilities|FlowControl|Delay (Variables|Default|GetAutoSpawnDelay))
  (CallFunction|EventSpawnActor))

(event Custom|Event_SpawnActor
  (bind _actortospawnclass (Variables|Default|GetActorToSpawnClass))
  ;[1 1 1] 生成Actor并配置自动生成和特殊配置
  (CallFunction|EventOpenCollision)
  (if (Utilities|IsValidClass _actortospawnclass)
    (bind _returnvalue (Game|SpawnActorfromClass _actortospawnclass (Transformation|GetWorldTransform (Variables|Default|GetDefaultSceneRoot)) "Undefined" 0 0))
    (bind _output_get (Variables|Default|SetActorToSpawn _returnvalue))
    (Utilities|IsValid _output_get
      (:Is%20Valid
        (Networking|SetReplicates _output_get true)
        (Game|BindEventtoOnDestroyed _output_get (delegate Custom|Event_OnActorDestroyed))
        ;;[1 1 1] 新方法自动关闭碰撞，但是产生耦合，应该新开个蓝图接口。。
        (Class|CanbePickUp|BindbePickUp(Message) (Variables|Default|GetActorToSpawn) self)))))

(event Custom|Event_ClearSelf
  ;[1 1 1] 自动关闭碰撞（废弃，但目前没有好的解耦的方法）
  (CallFunction|EventCloseCollision)
  (Variables|Default|SetActorToSpawn 0))

(event Custom|Event_CloseCollision
  (Collision|SetCollisionEnabled (Variables|Default|GetCollisionSphere) "NoCollision")
  (Variables|Default|SetIsOpenCollision false)
  (Variables|Default|SetActorToSpawn 0))

(event Custom|Event_OpenCollision
  (Collision|SetCollisionEnabled (Variables|Default|GetCollisionSphere) "QueryOnly")
  (Variables|Default|SetIsOpenCollision true))

(event EventBeginPlay
  ;[1 1 1] 生成Actor并配置自动生成和特殊配置
  (CallFunction|EventSpawnActor))

(fn ConstructionScript)

(fn OnRepIsOpenCollision
  (if (Variables|Default|GetIsOpenCollision)
    (Collision|SetCollisionEnabled (Variables|Default|GetCollisionSphere) "QueryOnly")
    (else
      (Collision|SetCollisionEnabled (Variables|Default|GetCollisionSphere) "NoCollision"))))