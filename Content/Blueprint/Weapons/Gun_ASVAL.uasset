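; ASVAL gun Blueprint: a hitscan weapon with high damage, a long fire cooldown and a small magazine, configured in its Construction Script.
; Fire spends a round, line-traces on the Camera channel with debug drawing, spawns effects and applies distance-based damage to Pawns, returning true only then.
; An empty magazine plays a sound; ReloadBullet moves one reserve round per call but never the last.
; The spread coefficient input is unused.
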(event EventBeginPlay
  (|CallParentFunction) ; 此节点被禁用，将不会被调用。\n从引脚连出引线来编译功能。
)

(event Collision|EventActorBeginOverlap
  (params (OtherActor :type Actor%20Object%20Reference))
  (|CallParentFunction OtherActor) ; 此节点被禁用，将不会被调用。\n从引脚连出引线来编译功能。
)

(event EventTick
  (params (DeltaSeconds :type Float%20%28single-precision%29))
  (|CallParentFunction DeltaSeconds) ; 此节点被禁用，将不会被调用。\n从引脚连出引线来编译功能。
)

(fn ConstructionScript
  (|CallParentFunction)
  (Utilities|FlowControl|Sequence
    (:then_0
      (Variables|Default|SetBulletType "NewEnumerator0")
      (Variables|Default|SetGunType "NewEnumerator2")
      (Variables|Default|SetFullDamageDistance 5e+03)
      (Variables|Default|SetFireCD 2.5)
      (Variables|Default|SetBaseDamage 1.5e+02)
      (Variables|Default|SetValidShootDistance 2e+04))
    (:then_1
      (Variables|Default|SetRemainAmorAmount 30)
      (Variables|Default|SetMagazineCapacityAmount 5)
      (Variables|Default|SetNowMagazineAmorAmount 5))
    (:then_2
      (Variables|Default|SetEquipSocketName "Weapon_AK47")
      (Variables|Default|SetGunName "ASVAL")
      (Variables|Default|SetReloadPlayTimes 1.2))))

(fn Fire
  (params (ShootDirect :type Vector :default "0, 0, 0") (StartLocation :type Vector :default "0, 0, 0") (DistrubCoefficient :type Float%20%28single-precision%29))
  (|CollapseGraph_0_2 ShootDirect StartLocation StartLocation StartLocation
    (:CastFailed
      (return false))
    (:then
      (return true))
    (:then2
      (return false))))

(fn ReloadBullet
  (if (and (> (Variables|Default|GetRemainAmorAmount) 1) (> (- (Variables|Default|GetMagazineCapacityAmount) (Variables|Default|GetNowMagazineAmorAmount)) 0))
    (Variables|Default|SetRemainAmorAmount (- (Variables|Default|GetRemainAmorAmount) 1))
    (Variables|Default|SetNowMagazineAmorAmount (+ (Variables|Default|GetNowMagazineAmorAmount) 1))
    (return 0)))