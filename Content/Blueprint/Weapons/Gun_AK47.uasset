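; AK47 weapon Blueprint that sets its stats, ammo, socket and name in the construction script and overrides hitscan firing.
; Fire spends a round, line-traces on the Camera channel with debug drawing, and spawns attack effects.
; Pawn hits take distance-based damage from CaculateRealDamage and return true; misses or an empty magazine, which plays a sound, return false.
; The DistrubCoefficient spread input is unused.
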(fn ConstructionScript
  (|CallParentFunction)
  (Utilities|FlowControl|Sequence
    (:then_0
      (Variables|Default|SetBulletType "NewEnumerator0")
      (Variables|Default|SetGunType "NewEnumerator0")
      (Variables|Default|SetFullDamageDistance 1.5e+03)
      (Variables|Default|SetFireCD 0.2)
      (Variables|Default|SetBaseDamage 2e+01)
      (Variables|Default|SetValidShootDistance 1e+04))
    (:then_1
      (Variables|Default|SetRemainAmorAmount 60)
      (Variables|Default|SetMagazineCapacityAmount 20)
      (Variables|Default|SetNowMagazineAmorAmount 20))
    (:then_2
      (Variables|Default|SetEquipSocketName "Weapon_AK47")
      (Variables|Default|SetGunName "AK47")
      (Variables|Default|SetReloadPlayTimes 1.0))))

(fn Fire
  (params (ShootDirect :type Vector :default "0, 0, 0") (StartLocation :type Vector :default "0, 0, 0") (DistrubCoefficient :type Float%20%28single-precision%29))
  (|CollapseGraph_0 ShootDirect StartLocation StartLocation StartLocation
    (:CastFailed
      (return false))
    (:then
      (return true))
    (:then2
      (return false))))