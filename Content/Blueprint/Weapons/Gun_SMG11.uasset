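; SMG11 submachine gun Blueprint, a hitscan weapon that sets its type, damage, range, ammo, socket and reload stats in the Construction Script.
; Fire spends a round, line-traces on the Camera channel with timed debug drawing, and spawns attack effects.
; Pawn hits take distance-adjusted damage and return true; misses return false, as does an empty magazine, which also plays a no-ammo sound.
; The DistrubCoefficient input is unused, so shots have no spread here.
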(event EventBeginPlay
  (|CallParentFunction) ; 此节点被禁用，将不会被调用。\n从引脚连出引线来编译功能。
)

(event Collision|EventActorBeginOverlap
  (params (OtherActor :type Actor%20Object%20Reference))
  (|CallParentFunction OtherActor) ; 此节点被禁用，将不会被调用。\n从引脚连出引线来编译功能。
)

(event EventTick
  (params (DeltaSeconds :type Float%20%28single-precision%29))
  (|CallParentFunction DeltaSeconds) ; 此节点被禁用，将不会被调用。\n从引脚连出引线来编译功能。
)

(fn ConstructionScript
  (|CallParentFunction)
  (Utilities|FlowControl|Sequence
    (:then_0
      (Variables|Default|SetBulletType "NewEnumerator1")
      (Variables|Default|SetGunType "NewEnumerator1")
      (Variables|Default|SetFullDamageDistance 8e+02)
      (Variables|Default|SetFireCD 0.1)
      (Variables|Default|SetBaseDamage 2e+01)
      (Variables|Default|SetValidShootDistance 6e+03))
    (:then_1
      (Variables|Default|SetRemainAmorAmount 180)
      (Variables|Default|SetMagazineCapacityAmount 25)
      (Variables|Default|SetNowMagazineAmorAmount 25))
    (:then_2
      (Variables|Default|SetEquipSocketName "Weapon_AK47")
      (Variables|Default|SetGunName "SMG11")
      (Variables|Default|SetReloadPlayTimes 1.5))))

(fn Fire
  (params (ShootDirect :type Vector :default "0, 0, 0") (StartLocation :type Vector :default "0, 0, 0") (DistrubCoefficient :type Float%20%28single-precision%29))
  (|CollapseGraph_0_2 ShootDirect StartLocation StartLocation StartLocation
    (:CastFailed
      (return false))
    (:then
      (return true))
    (:then2
      (return false))))