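; Default AI controller that runs BT_Default and drives gun firing for Character_AI pawns.
; AI perception updates write the IsSeePlayer blackboard key when the sensed actor is a living Character_RobHat.
; Start and stop fire events toggle a looping timer at the gun's fire cooldown, with a negative start delay cancelling the first wait.
; Each tick of that timer fires unless the pawn is dead or reloading.
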(event OnTargetPerceptionUpdated(AIPerception)
  (params (Actor :type Actor%20Object%20Reference) (Stimulus :type AI%20Stimulus%20Structure))
  (bind _ascharacter_rob_hat (Utilities|Casting|CastToCharacter_RobHat Actor))
  (if (not (Variables|/Game/Blueprint/Character_RobHat.Character_RobHat_C|GetbIsDied _ascharacter_rob_hat))
    (AI|Components|Blackboard|SetValueasBool (AI|GetBlackboard 0) (Utilities|Name|MakeLiteralName "IsSeePlayer") (.bSuccessfullySensed (Utilities|Struct|BreakAIStimulus Stimulus)))))

(event Custom|Event_StartFire
  ;[1 1 1] 开火
  (if (not (Variables|Default|GetIsFiring))
    (Variables|Default|SetIsFiring true)
    (bind _ascharacter_ai (Utilities|Casting|CastToCharacter_AI (Pawn|GetControlledPawn)))
    (bind _returnvalue (Utilities|Time|SetTimerbyFunctionName 0 "Event_Fire" (Variables|/Game/Blueprint/InterfaceAndBase/BaseGun.BaseGun_C|GetFireCD (Variables|/Game/Blueprint/AI/Character_AI.Character_AI_C|GetNowUseGun _ascharacter_ai)) true (- 0.0 (Variables|/Game/Blueprint/InterfaceAndBase/BaseGun.BaseGun_C|GetFireCD (Variables|/Game/Blueprint/AI/Character_AI.Character_AI_C|GetNowUseGun _ascharacter_ai)))))))

(event Custom|Event_StopFire
  ;[1 1 1] 开火
  (if (Variables|Default|GetIsFiring)
    (Variables|Default|SetIsFiring false)
    (Utilities|Time|ClearandInvalidateTimerbyHandle (stale Custom|Event_StartFire _returnvalue))))

(event Custom|Event_Fire
  ;[1 1 1] 开火
  (bind _ascharacter_ai (Utilities|Casting|CastToCharacter_AI (Pawn|GetControlledPawn)))
  (if (not (Variables|/Game/Blueprint/AI/Character_AI.Character_AI_C|GetbIsDied _ascharacter_ai))
    (if (not (Variables|/Game/Blueprint/AI/Character_AI.Character_AI_C|GetIsReBulleting _ascharacter_ai))
      (Default|EventOpenFire _ascharacter_ai))))

(event EventBeginPlay
  (AI|RunBehaviorTree "/Game/Blueprint/AI/BT_Default.BT_Default"))

(fn ConstructionScript)