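; AI-controlled enemy character that fights the player with a spawned, socket-attached gun and shows a world-space health bar.
; Its controller calls the fire event, which plays hip or ironsight montages and shoots toward the player, or reloads on an empty magazine.
; Damage reveals the bar and focuses the AI on the player.
; Health, death and failed-shot sight loss are written to the Blackboard.
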(event Custom|Event_OpenFire
  (bind _nowusegun (Variables|Weapon|GetNowUseGun))
  (bind _mesh (Variables|Character|GetMesh))
  ;[1 1 1] Pawn开火，由controller调用并控制
  (if (not (Variables|Default|GetbIsDied))
    (|IfPlayerLive
      (:else
        (if (<= (Variables|/Game/Blueprint/InterfaceAndBase/BaseGun.BaseGun_C|GetNowMagazineAmorAmount _nowusegun) 0)
          (CallFunction|EventReBullet)
          (else
            (if (Variables|Default|GetbIsAimMode)
              (Animation|Montage|PlayMontage _mesh "/Game/MyAsset/Animation/Fire_Rifle_Ironsights_Montage.Fire_Rifle_Ironsights_Montage"
                (:then
                  _))
              (else
                (Animation|Montage|PlayMontage _mesh "/Game/MyAsset/Animation/Fire_Rifle_Hip_Montage.Fire_Rifle_Hip_Montage"
                  (:then
                    _))))
            (bind _bishitpawn (Default|Fire _nowusegun (- (Transformation|GetActorLocation (Game|GetPlayerCharacter 0)) (Transformation|GetActorLocation)) (Transformation|GetSocketLocation (Variables|Character|GetMesh) "Weapon_AK47") 0.0))
            (if (not _bishitpawn)
              (AI|Components|Blackboard|SetValueasBool (AI|GetBlackboard 0) (Utilities|Name|MakeLiteralName "IsSeePlayer") false)
              (Pawn|Components|CharacterMovement|DisableMovement (Variables|Character|GetCharacterMovement)))))))))

(event Custom|Event_ReBullet
  (bind _nowusegun (Variables|Weapon|GetNowUseGun))
  ;[1 1 1] 换弹
  (Variables|Default|SetIsReBulleting true)
  (Utilities|IsValid _nowusegun
    (:Is%20Valid
      (Animation|Montage|PlayMontage (Variables|Character|GetMesh) "/Game/MyAsset/Animation/Reload_Rifle_Hip_Montage.Reload_Rifle_Hip_Montage" (Variables|/Game/Blueprint/InterfaceAndBase/BaseGun.BaseGun_C|GetReloadPlayTimes _nowusegun)
        (:then
          (Default|EventPlayReloadBulletEffect _nowusegun))
        (:OnCompleted
          (Class|GunBaseInterface|ReloadBullet(Message) _nowusegun)
          (Variables|Default|SetIsReBulleting false))))))

(event Custom|Event_AI_Init
  (bind _maxhealth (Variables|Default|GetMaxHealth))
  ;[1 1 1] 初始化
  (Variables|GamePlay|SetHealthCeiling _maxhealth)
  (Variables|GamePlay|SetNowHealth _maxhealth)
  (bind _returnvalue (Game|SpawnActorfromClass (Variables|Default|GetGunClass) (Transformation|GetActorTransform) "Undefined" 0 0))
  (bind _output_get (Variables|Weapon|SetNowUseGun _returnvalue))
  (Default|EquiptoMeshCompbySocket _output_get (Variables|Character|GetMesh))
  (Actor|SetOwner _output_get self)
  (Game|BindEventtoOnDestroyed (delegate Custom|自定义事件_0)))

(event Custom|自定义事件_0
  (params (DestroyedActor :type Actor%20Object%20Reference))
  ;[1 1 1] 初始化
  (Actor|DestroyActor (Variables|Weapon|GetNowUseGun)))

(event Custom|Event_ShowHealthBar
  ;[1 1 1] 更新血量UI
  (Rendering|SetVisibility (Variables|Default|GetHealthRoot) true true))

(event Custom|Event_UpdateHealthBar
  (bind _healthceiling (Variables|GamePlay|GetHealthCeiling))
  (bind _nowhealth (Variables|GamePlay|GetNowHealth))
  ;[1 1 1] 更新血量UI
  (if (Rendering|IsVisible (Variables|Default|GetHealthRoot))
    (bind _aswidget_health_bar (Utilities|Casting|CastToWidget_HealthBar (UserInterface|GetWidget (Variables|Default|GetHealthBar))))
    (Progress|SetPercent (Variables|/Game/Blueprint/UI/Game/Widget_HealthBar.Widget_HealthBar_C|GetProgressBar_65 _aswidget_health_bar) (/ (Math|Conversions|ToFloat(Integer) _nowhealth) (Math|Conversions|ToFloat(Integer) _healthceiling)))
    (Rendering|Components|TextRender|SetText (Variables|Default|GetTextHealth) (Utilities|Text|FormatText "{a} / {b}" _nowhealth _healthceiling))))

(event Custom|Event_PickHealth
  (params (Value :type Integer))
  (bind _healthceiling (Variables|GamePlay|GetHealthCeiling))
  ;[1 1 1] 回血
  (if (> (+ Value (Variables|GamePlay|GetNowHealth)) _healthceiling)
    (Variables|GamePlay|SetNowHealth _healthceiling)
    (else
      (Variables|GamePlay|SetNowHealth (+ Value (Variables|GamePlay|GetNowHealth)))))
  (CallFunction|WhenHealthChange))

(event Custom|Event_Anim_SetAimOffset
  ;[1 1 1] 设置瞄准偏移
  (Variables|Default|SetPitch_AimOffset (.Pitch (Math|Rotator|BreakRotator (Math|Interpolation|RInterpTo (Math|Rotator|Delta(Rotator) (Math|Rotator|MakeRotator 0.0 (.Pitch (Math|Rotator|BreakRotator (Pawn|GetControlRotation :!class /Script/Engine.Pawn))) 0.0) (Math|Rotator|MakeRotator 0.0 (.Pitch (Math|Rotator|BreakRotator (Transformation|GetActorRotation))) 0.0)) (Math|Rotator|MakeRotator 0.0 (Variables|Default|GetPitch_AimOffset) 0.0) 0.01 2e+01)))))

(event EventBeginPlay
  ;[1 1 1] 初始化
  (CallFunction|EventAIInit)
  (Rendering|SetVisibility (Variables|Default|GetHealthRoot) false true)
  (CallFunction|WhenHealthChange))

(event Game|Damage|EventAnyDamage
  (params (Damage :type Float%20%28single-precision%29) (DamageType :type Damage%20Type%20Object%20Reference) (InstigatedBy :type Controller%20Object%20Reference) (DamageCauser :type Actor%20Object%20Reference))
  (bind _returnvalue (Math|Float|Truncate Damage))
  ;[1 1 1] AI受伤
  (if (not (Variables|Default|GetbIsDied))
    (CallFunction|EventShowHealthBar)
    (AI|SetFocus (AI|GetAIController self) (Game|Player|GetPlayerPawn 0))
    (if (> (Variables|GamePlay|GetNowHealth) _returnvalue)
      (Variables|GamePlay|SetNowHealth (- (Variables|GamePlay|GetNowHealth) _returnvalue))
      (else
        (Variables|GamePlay|SetNowHealth 0)
        (Variables|Default|SetbIsDied true)
        (AI|Components|Blackboard|SetValueasBool (AI|GetBlackboard 0) (Utilities|Name|MakeLiteralName "IsDied") true)))
    (CallFunction|WhenHealthChange)))

(event EventTick
  (params (DeltaSeconds :type Float%20%28single-precision%29))
  (bind _healthroot (Variables|Default|GetHealthRoot))
  ;[1 1 1] 血条自动旋转
  (if (Rendering|IsVisible _healthroot)
    (Transformation|SetWorldRotation _healthroot (|FaceToPlayer) false false)))

(fn ConstructionScript)

(fn WhenHealthChange
  (CallFunction|EventUpdateHealthBar)
  (Class|BlackboardComponent|SetValueasInt (AI|GetBlackboard 0) (Utilities|Name|MakeLiteralName "Health") (Variables|GamePlay|GetNowHealth)))