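; Health pack pickup actor that grants health to the character that picks it up, then destroys itself.
; PickUp gives HealthValue to a Character_RobHat or double that to a Character_AI through EventPickHealth, and does nothing for other pawns.
; BindbePickUp hooks OnDestroyed to call EventCloseCollision on the supplied SpawnActor, a callback the author flags as ugly coupling.
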(event Custom|自定义事件_0
  (params (DestroyedActor :type Actor%20Object%20Reference))
  ;[1 1 1] 丑陋的耦合的回调
  (Default|EventCloseCollision (stale EventBindbePickUp SpawnActor)))

(event EventBeginPlay)

(event Collision|EventActorBeginOverlap
  (params (OtherActor :type Actor%20Object%20Reference)))

(event EventTick
  (params (DeltaSeconds :type Float%20%28single-precision%29)))

(event EventBindbePickUp
  (params (SpawnActor :type Auto%20Spawn%20Actor%20New%20Object%20Reference))
  ;[1 1 1] 丑陋的耦合的回调
  (Game|BindEventtoOnDestroyed (delegate Custom|自定义事件_0)))

(fn ConstructionScript)

(fn PickUp
  (params (PawnToPickUp :type Pawn%20Object%20Reference))
  (bind _ascharacter_rob_hat (Utilities|Casting|CastToCharacter_RobHat PawnToPickUp)
    (:then
      (Default|EventPickHealth _ascharacter_rob_hat (Variables|Default|GetHealthValue)))
    (:CastFailed
      (bind _ascharacter_ai (Utilities|Casting|CastToCharacter_AI PawnToPickUp))
      (Default|EventPickHealth _ascharacter_ai (* (Variables|Default|GetHealthValue) 2))))
  (Actor|DestroyActor)
  (return true))