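; Base gun actor for child weapons to extend, covering pickup, ammo, damage falloff and hit effects, with Fire left as an overridable stub.
; PickUp registers with Character_RobHat, attaches to a mesh socket, sets ownership and fires OnBePickUp, which a bound spawner uses to close collision.
; Reserve ammo refills the magazine, and damage falls linearly beyond full-damage range.
; Shot effects spawn a bullet-hole decal, hit particle and 2D fire sound.
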(event Custom|Event_PlayReloadBulletEffect
  ;[1 1 1] 换弹声音
  (Audio|SpawnSoundatLocation (Variables|EffectSource|GetSound_Reload) (Transformation|GetActorLocation (Components|GetOwner)) "0, 0, 0" 1.0 1.0 0.0 0 0))

(event Custom|自定义事件_0
  ;[1 1 1] 关闭生成器的碰撞，这样实现会导致耦合，但是没找到在蓝图接口传入代理事件的办法
  (Default|EventCloseCollision (stale EventBindbePickUp SpawnActor)))

(event EventBeginPlay)

(event Collision|EventActorBeginOverlap
  (params (OtherActor :type Actor%20Object%20Reference)))

(event EventTick
  (params (DeltaSeconds :type Float%20%28single-precision%29)))

(event EventAddAmor
  (params (AmorAmount :type Integer))
  ;[1 1 1] 补充子弹
  (Variables|GunAttributes|SetRemainAmorAmount (+ AmorAmount (Variables|GunAttributes|GetRemainAmorAmount))))

(event EventBindbePickUp
  (params (SpawnActor :type Auto%20Spawn%20Actor%20New%20Object%20Reference))
  ;[1 1 1] 关闭生成器的碰撞，这样实现会导致耦合，但是没找到在蓝图接口传入代理事件的办法
  (EventDispatchers|BindEventtoOnbePickUp (delegate Custom|自定义事件_0)))

(fn ConstructionScript)

(fn SpawnAttackEffect
  (params (StartLocation :type Vector) (HitPack :type Hit%20Result%20Structure))
  (bind (_bblockinghit _binitialoverlap _time _distance _location _impactpoint _normal _impactnormal _physmat _hitactor _hitcomponent) (Collision|BreakHitResult HitPack))
  (bind _returnvalue (Math|Rotator|MakeRotfromX _normal))
  ;[1 1 1] 开枪音效，爆炸效果和弹孔
  (Rendering|Decal|SpawnDecalatLocation (Variables|EffectSource|GetBulletHoleDecal) "1.000000,4.000000,4.000000" _location _returnvalue 6.0)
  (Effects|SpawnEmitterAttached (Variables|EffectSource|GetHitParticle) _hitcomponent "None" _location _returnvalue "0.200000,0.200000,0.200000" "KeepWorldPosition")
  (Audio|PlaySound2D (Variables|EffectSource|GetFireSoundWave) 0.25 1.0 0.0 0 0))

(fn BaseGunAutoGenFunc
  (params (DestroyedActor :type Actor%20Object%20Reference))
  (Actor|DestroyActor self))

(fn CaculateRealDamage
  (params (ShootDistance :type Float%20%28single-precision%29))
  (bind _fulldamagedistance (Variables|GunAttributes|GetFullDamageDistance))
  (bind _basedamage (Variables|GunAttributes|GetBaseDamage))
  ;[1 1 1] 超出有效射程伤害线性衰减
  (if (< ShootDistance _fulldamagedistance)
    (return _basedamage)
    (else
      (return (* _basedamage (- 1.0 (/ (- ShootDistance _fulldamagedistance) (- (Variables|GunAttributes|GetValidShootDistance) (Variables|GunAttributes|GetFullDamageDistance)))))))))

(fn EquiptoMeshCompbySocket
  (params (CharacterMeshComp :type Skeletal%20Mesh%20Component%20Object%20Reference))
  (bind _gunmesh (Variables|Default|GetGunMesh))
  ;[1 1 1] 装备附加到mesh
  (Utilities|IsValid _gunmesh
    (:Is%20Valid
      (Utilities|IsValid CharacterMeshComp
        (:Is%20Valid
          (bind _returnvalue (Transformation|AttachComponentToComponent _gunmesh CharacterMeshComp (Variables|GunAttributes|GetEquipSocketName) "SnapToTarget" "SnapToTarget" "SnapToTarget" true))
          (return _returnvalue))))))

(fn Fire
  (params (ShootDirect :type Vector :default "0, 0, 0") (StartLocation :type Vector :default "0, 0, 0") (DistrubCoefficient :type Float%20%28single-precision%29))
  ;[1 1 1] 交给子类重载
  (return false))

(fn IsMatchAmor
  (params (AmorActor :type Base%20Bullet%20Object%20Reference))
  (return (Utilities|Enum|Equal(Enum) (Variables|/Game/Blueprint/InterfaceAndBase/BaseBullet.BaseBullet_C|GetBulletType AmorActor) (Variables|GunAttributes|GetBulletType))))

(fn PickUp
  (params (PawnToPickUp :type Pawn%20Object%20Reference))
  (bind _ascharacter_rob_hat (Utilities|Casting|CastToCharacter_RobHat PawnToPickUp))
  (Default|EventPickGun _ascharacter_rob_hat self)
  (Game|BindEventtoOnDestroyed _ascharacter_rob_hat (EventDispatchers|CreateEvent :!event BaseGunAutoGenFunc))
  (bind _issuccess (CallFunction|EquiptoMeshCompbySocket (Variables|/Script/Engine.Character|GetMesh _ascharacter_rob_hat)))
  (Default|CallOnbePickUp)
  (Actor|SetOwner PawnToPickUp)
  (return _issuccess))

(fn ReloadBullet
  ;[1 1 1] 用剩余子弹补充弹匣子弹
  (if (> (Variables|GunAttributes|GetRemainAmorAmount) (- (Variables|GunAttributes|GetMagazineCapacityAmount) (Variables|GunAttributes|GetNowMagazineAmorAmount)))
    (Variables|GunAttributes|SetRemainAmorAmount (- (Variables|GunAttributes|GetRemainAmorAmount) (- (Variables|GunAttributes|GetMagazineCapacityAmount) (Variables|GunAttributes|GetNowMagazineAmorAmount))))
    (Variables|GunAttributes|SetNowMagazineAmorAmount (Variables|GunAttributes|GetMagazineCapacityAmount))
    (return (- (Variables|GunAttributes|GetMagazineCapacityAmount) (Variables|GunAttributes|GetNowMagazineAmorAmount)))
    (else
      ;;[1 1 1] 剩余子弹不够补满弹匣
      (Variables|GunAttributes|SetNowMagazineAmorAmount (+ (Variables|GunAttributes|GetRemainAmorAmount) (Variables|GunAttributes|GetNowMagazineAmorAmount)))
      (Variables|GunAttributes|SetRemainAmorAmount 0)
      (return (Variables|GunAttributes|GetRemainAmorAmount)))))