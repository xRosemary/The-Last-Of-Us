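; PC_Lobby is the lobby player controller, linking each player's lobby UI to GM_Lobby.
; On BeginPlay it reads PlayerInfo from GameInstance_Main, registers it with the game mode, shows UI_Lobby and requests an all-player update.
; Other events forward info changes to GM_Lobby and push player lists into the widget.
; It also shows the loading screen and handles leaving by destroying the session and opening Map_Start.
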(event Custom|Event_Init
  ;[1 1 1] 初始化
  (bind _asgame_instance_main (Utilities|Casting|CastToGameInstance_Main (Game|GetGameInstance)))
  (bind _output_get (Variables|Default|SetPlayerInfo (Variables|/Game/Blueprint/GameController/GameInstance_Main.GameInstance_Main_C|GetPlayerInfo _asgame_instance_main)))
  (CallFunction|EventAddPlayerInfo _output_get)
  (CallFunction|EventShowLobbyUI))

(event Custom|Event_ShowLobbyUI
  ;[1 1 1] 创建LobbyUI
  (Variables|Default|SetbShowMouseCursor true)
  (bind _returnvalue (UserInterface|CreateWidget "/Game/Blueprint/UI/Lobby/UI_Lobby.UI_Lobby_C" self))
  (bind _output_get (Variables|Default|SetUI_Lobby _returnvalue))
  (UserInterface|Viewport|AddtoViewport _output_get 0)
  (Input|SetInputModeGameandUI self _output_get "DoNotLock" true)
  (CallFunction|EventUpdatePlayer))

(event Custom|Event_ShowLoadingUI
  ;[1 1 1] 显示加载页面
  (bind _returnvalue (UserInterface|CreateWidget "/Game/Blueprint/UI/Game/UI_GameLoading.UI_GameLoading_C" self))
  (UserInterface|Viewport|AddtoViewport _returnvalue 0))

(event Custom|Event_LeaveRome
  ;[1 1 1] 退出游戏房间
  (|DestroySession self
    (:OnSuccess
      (Game|OpenLevel(byName) "Map_Start"))))

(event Custom|Event_UpdateSelfLobbyUI
  (params (PlayerInfoList :type Array%20of%20Player%20Info%20Struct%20Structures))
  ;[1 1 1] 更新客户端LobbyUI
  (Default|EventUpdateAllLobbyInfo (Variables|Default|GetUI_Lobby) PlayerInfoList))

(event Custom|Event_UpdatePlayerInfo
  (params (PlayerInfo :type Player%20Info%20Struct%20Structure))
  ;[1 1 1] 更新玩家信息
  (bind _asgm_lobby (Utilities|Casting|CastToGM_Lobby (Game|GetGameMode)))
  (Default|EventUpdatePlayerInfo _asgm_lobby PlayerInfo)
  (Variables|Default|SetPlayerInfo PlayerInfo))

(event Custom|Event_UpdatePlayer
  ;[1 1 1] 更新全部玩家
  (bind _asgm_lobby (Utilities|Casting|CastToGM_Lobby (Game|GetGameMode)))
  (Default|EventUpdateAllPlayer _asgm_lobby))

(event Custom|Event_AddPlayerInfo
  (params (PlayerInfo :type Player%20Info%20Struct%20Structure))
  ;[1 1 1] GameMode添加自己的PlayerInfo
  (bind _asgm_lobby (Utilities|Casting|CastToGM_Lobby (Game|GetGameMode)))
  (Default|EventAddPlayerInfo _asgm_lobby PlayerInfo))

(event EventBeginPlay
  ;[1 1 1] 初始化
  (CallFunction|EventInit))

(fn ConstructionScript)