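; Lobby game mode that tracks connected players and moves the session to Map_Online through ServerTravel.
; On login it records the controller and possesses a new Character_Lobby at the first PlayerStart found.
; It keeps player info in an array assumed index-aligned with controllers, removing entries on logout and replacing updates by name.
; Logouts and info updates push the list to every PC_Lobby to refresh lobby UI.
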(event Custom|Event_SpawnPlayer
  (params (PlayerController :type Player%20Controller%20Object%20Reference))
  (bind _returnvalue (Pawn|GetControlledPawn PlayerController))
  ;[1 1 1] 生成玩家Pawn
  (Utilities|IsValid _returnvalue
    (:Is%20Valid
      (Actor|DestroyActor _returnvalue))
    (:Is%20Not%20Valid
      _))
  (bind _outactors (Actor|GetAllActorsOfClass "/Script/Engine.PlayerStart"))
  (bind _returnvalue_2 (Game|SpawnActorfromClass "/Game/Blueprint/Character_Lobby.Character_Lobby_C" (Transformation|GetActorTransform (Utilities|Array|Get(acopy) _outactors)) "Undefined" 0 0))
  (Pawn|Possess PlayerController _returnvalue_2))

(event Custom|Event_StartGame
  ;[1 1 1] 场景漫游开始游戏
  (Development|ExecuteConsoleCommand "ServerTravel Map_Online" (Game|GetPlayerController 0)))

(event Custom|Event_UpdateAllPlayer
  ;[1 1 1] 将房间用户UI更新
  (for _array_element (Variables|Default|GetPlayerList)
    (bind _aspc_lobby (Utilities|Casting|CastToPC_Lobby _array_element))
    (Default|EventUpdateSelfLobbyUI _aspc_lobby (Variables|Default|GetPlayerInfoList))))

(event Custom|Event_AddPlayerInfo
  (params (PlayerInfo :type Player%20Info%20Struct%20Structure))
  ;[1 1 1] 添加到玩家信息数组
  (Utilities|Array|Add (Variables|Default|GetPlayerInfoList) PlayerInfo))

(event Custom|Event_UpdatePlayerInfo
  (params (PlayerInfo :type Player%20Info%20Struct%20Structure))
  (bind _tempplayerinfolist (Variables|Default|GetTempPlayerInfoList))
  ;[1 1 1] 更新需要更新的玩家的Info
  (Utilities|Array|Clear (Variables|Default|GetTempPlayerInfoList))
  (for _array_element (Variables|Default|GetPlayerInfoList)
    (if (Utilities|Enum|Equal(Enum) (.Name (Utilities|Struct|BreakPlayerInfoStruct _array_element)) (.Name (Utilities|Struct|BreakPlayerInfoStruct PlayerInfo)))
      (Utilities|Array|Add _tempplayerinfolist PlayerInfo)
      (else
        (Utilities|Array|Add _tempplayerinfolist _array_element))))
  (Variables|Default|SetPlayerInfoList (Variables|Default|GetTempPlayerInfoList))
  (CallFunction|EventUpdateAllPlayer))

(event EventOnLogout
  (params (ExitingController :type Controller%20Object%20Reference))
  ;[1 1 1] 玩家登出时
  (Networking|SwitchHasAuthority
    (:Authority
      (for (_array_element _array_index) (Variables|Default|GetPlayerList)
        (if (== _array_element ExitingController)
          (Utilities|Array|RemoveItem (Variables|Default|GetPlayerList) _array_element)
          (Utilities|Array|RemoveIndex (Variables|Default|GetPlayerInfoList) _array_index)))
      (CallFunction|EventUpdateAllPlayer))))

(event EventPostLogin
  (params (NewPlayer :type Player%20Controller%20Object%20Reference))
  ;[1 1 1] 玩家登录进Lobby时
  (Networking|SwitchHasAuthority
    (:Authority
      (Utilities|Array|Add (Variables|Default|GetPlayerList) NewPlayer)
      (CallFunction|EventSpawnPlayer NewPlayer))))

(fn ConstructionScript)