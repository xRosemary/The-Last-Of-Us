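; GM_PlayWithAI is the game mode for the play-with-AI mode, handling player respawn and game over.
; Event_RebornPawn accepts only a PC_PlayWithAI, destroys its current pawn, spawns a Character_RobHat at the first PlayerStart found, possesses it and sets walking movement.
; Event_GameOver shows the mouse cursor and creates the UI_GameOver widget for that player, with no AddToViewport call in this graph.
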(event Custom|Event_GameOver
  (params (PC :type Player%20Controller%20Object%20Reference))
  (Variables|/Script/Engine.PlayerController|SetbShowMouseCursor PC true)
  (UserInterface|CreateWidget "/Game/Blueprint/UI/Game/UI_GameOver.UI_GameOver_C" PC))

(event Custom|Event_RebornPawn
  (params (PC :type Player%20Controller%20Object%20Reference))
  (bind _returnvalue (Pawn|GetControlledPawn PC))
  ;[1 1 1] 复活
  (Utilities|Casting|CastToPC_PlayWithAI PC)
  (bind _outactors (Actor|GetAllActorsOfClass "/Script/Engine.PlayerStart"))
  (Utilities|IsValid _returnvalue
    (:Is%20Valid
      (Actor|DestroyActor _returnvalue))
    (:Is%20Not%20Valid
      _))
  (bind _returnvalue_2 (Game|SpawnActorfromClass "/Game/Blueprint/Character_RobHat.Character_RobHat_C" (Transformation|GetActorTransform (Utilities|Array|Get(acopy) _outactors)) "Undefined" 0 0))
  (Pawn|Possess PC _returnvalue_2)
  (Pawn|Components|CharacterMovement|SetMovementMode (Variables|/Script/Engine.Character|GetCharacterMovement _returnvalue_2) "MOVE_Walking" 0))

(event EventBeginPlay)

(event EventTick
  (params (DeltaSeconds :type Float%20%28single-precision%29)))

(fn ConstructionScript)