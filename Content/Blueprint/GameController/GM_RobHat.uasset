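; Game mode for a RobHat multiplayer match that runs the round, tracks kills and deaths, and picks the winner by most kills.
; PostLogin registers player controllers and spawns characters at indexed PlayerStarts, which respawns reuse.
; Looping one-second timers drive the start countdown, which enables walking, then the match countdown, shown only near the end.
; It pushes shared player stats and countdowns to every controller, then server-travels to the lobby after announcing the winner.
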(event Custom|Event_InitSapwnPlayer
  (params (PC :type Player%20Controller%20Object%20Reference))
  ;[1 1 1] 初始化玩家pawn
  (if (> (Utilities|Array|Length (Variables|Default|GetLoactionToSpawnList)) 0)
    (bind _aspc_rob_hat (Utilities|Casting|CastToPC_RobHat PC))
    (Utilities|IsValid (Pawn|GetControlledPawn _aspc_rob_hat)
      (:Is%20Valid
        (Transformation|SetActorTransform (Pawn|GetControlledPawn _aspc_rob_hat) (Transformation|GetActorTransform (Utilities|Array|Get(acopy) (Variables|Default|GetLoactionToSpawnList) (.playernumber (Variables|/Game/Blueprint/GameController/PC_RobHat.PC_RobHat_C|GetPlayerGameInfo _aspc_rob_hat))))))
      (:Is%20Not%20Valid
        (bind _returnvalue (Game|SpawnActorfromClass "/Game/Blueprint/Character_RobHat.Character_RobHat_C" (Transformation|GetActorTransform (Utilities|Array|Get(acopy) (Variables|Default|GetLoactionToSpawnList) (.playernumber (Variables|/Game/Blueprint/GameController/PC_RobHat.PC_RobHat_C|GetPlayerGameInfo _aspc_rob_hat)))) "Undefined" 0 0))
        (Pawn|Possess PC _returnvalue)))
    (else
      (bind _outactors (Actor|GetAllActorsOfClass "/Script/Engine.PlayerStart"))
      (Variables|Default|SetLoactionToSpawnList _outactors))))

(event Custom|Event_AddPlayerGameInfo
  (params (PlayerGameInfo :type Rob%20Hat%20Player%20Info%20Struct%20Structure))
  ;[1 1 1] PC调用，初始化info list
  (if (Math|Integer|InRange(Integer) (.PlayerNumber (Utilities|Struct|BreakRobHatPlayerInfoStruct PlayerGameInfo)) 0 3)
    (Utilities|Array|AddUnique (Variables|Default|GetPlayerGameInfoList) PlayerGameInfo)
    (CallFunction|EventUpdatePlayersAllGameInfo)))

(event Custom|Event_WhenGamePlayEnd
  ;[1 1 1] 通知玩家游戏结束，并且自动返回大厅
  (CallFunction|EventCaculateWinner)
  (Variables|Default|SetIsGamePlaying false)
  (for _array_element (Variables|Default|GetPlayerList)
    (Default|EventwhenGameEnd _array_element (Variables|Default|GetWinnerPlayer)))
  (Utilities|FlowControl|Delay 6.0)
  (Development|ExecuteConsoleCommand "ServerTravel Map_Lobby" (Game|GetPlayerController 0)))

(event Custom|Event_CaculateWinner
  ;[1 1 1] 计算胜利玩家
  (for _array_element (Variables|Default|GetPlayerGameInfoList)
    (if (> (.KillSum (Utilities|Struct|BreakRobHatPlayerInfoStruct _array_element)) (.KillSum (Utilities|Struct|BreakRobHatPlayerInfoStruct (Utilities|Array|Get(acopy) (Variables|Default|GetPlayerGameInfoList) (Variables|Default|GetWinnerPlayer)))))
      (Variables|Default|SetWinnerPlayer (.PlayerNumber (Utilities|Struct|BreakRobHatPlayerInfoStruct _array_element))))))

(event Custom|Event_UpdatePlayersAllGameInfo
  ;[1 1 1] 更新玩家的GameInfo
  (if (Variables|Default|GetIsGamePlaying)
    (for _array_element (Variables|Default|GetPlayerList)
      (Variables|/Game/Blueprint/GameController/PC_RobHat.PC_RobHat_C|SetAllPlayerGameInfo _array_element (Variables|Default|GetPlayerGameInfoList)))))

(event Custom|Event_UpdateOnesGameInfo
  (params (PlayerInfo :type Rob%20Hat%20Player%20Info%20Struct%20Structure))
  (bind _playernumber (Utilities|Struct|BreakRobHatPlayerInfoStruct PlayerInfo))
  ;[1 1 1] 更新玩家的GameInfo
  (if (Variables|Default|GetIsGamePlaying)
    (if (Math|Integer|InRange(Integer) _playernumber 0 3)
      (Utilities|Array|SetArrayElem (Variables|Default|GetPlayerGameInfoList) _playernumber PlayerInfo true)
      (CallFunction|EventUpdatePlayersAllGameInfo))))

(event Custom|Event_UpdateKDA
  (params (KillerPC :type PC%20Rob%20Hat%20Object%20Reference) (DiedPC :type PC%20Rob%20Hat%20Object%20Reference))
  (bind _playergameinfo (Variables|/Game/Blueprint/GameController/PC_RobHat.PC_RobHat_C|GetPlayerGameInfo DiedPC))
  (bind _playergameinfo_2 (Variables|/Game/Blueprint/GameController/PC_RobHat.PC_RobHat_C|GetPlayerGameInfo KillerPC))
  ;[1 1 1] 被kill的人的PC调用，更新双方KDA
  (Utilities|Struct|SetmembersinRobHatPlayerInfoStruct _playergameinfo_2 (+ (.KillSum (Utilities|Struct|BreakRobHatPlayerInfoStruct _playergameinfo_2)) 1))
  (Utilities|Struct|SetmembersinRobHatPlayerInfoStruct _playergameinfo (+ (.DeadSum (Utilities|Struct|BreakRobHatPlayerInfoStruct _playergameinfo)) 1)))

(event Custom|Event_RebornPawn
  (params (PC :type Player%20Controller%20Object%20Reference))
  ;[1 1 1] 复活
  (bind _aspc_rob_hat (Utilities|Casting|CastToPC_RobHat PC))
  (Utilities|IsValid (Pawn|GetControlledPawn _aspc_rob_hat)
    (:Is%20Valid
      (Actor|DestroyActor (Pawn|GetControlledPawn _aspc_rob_hat)))
    (:Is%20Not%20Valid
      _))
  (bind _returnvalue (Game|SpawnActorfromClass "/Game/Blueprint/Character_RobHat.Character_RobHat_C" (Transformation|GetActorTransform (Utilities|Array|Get(acopy) (Variables|Default|GetLoactionToSpawnList) (.playernumber (Variables|/Game/Blueprint/GameController/PC_RobHat.PC_RobHat_C|GetPlayerGameInfo _aspc_rob_hat)))) "Undefined" 0 0))
  (Pawn|Possess _aspc_rob_hat _returnvalue)
  (Pawn|Components|CharacterMovement|SetMovementMode (Variables|/Script/Engine.Character|GetCharacterMovement _returnvalue) "MOVE_Walking" 0))

(event Custom|Event_Timer_StartGame
  ;[1 1 1] 进入Level后，游戏同步倒计时结束才允许移动
  (Variables|Default|SetTimeCountDown (Variables|Default|GetTimeWaitStart))
  (CallFunction|EventUpdateAllCountDown)
  (if (> (Variables|Default|GetTimeWaitStart) 0)
    (Variables|Default|SetTimeWaitStart (- (Variables|Default|GetTimeWaitStart) 1))
    (else
      (Utilities|Time|ClearandInvalidateTimerbyHandle (stale EventBeginPlay _returnvalue))
      (CallFunction|EventwhenGameStart))))

(event Custom|Event_UpdateAllCountDown
  ;[1 1 1] 将TimeCountDown同步到玩家屏幕
  (for _array_element (Variables|Default|GetPlayerList)
    (Default|EventGetSertveCountDown _array_element (Variables|Default|GetTimeCountDown))))

(event Custom|Event_WhenGameStart
  ;[1 1 1] 游戏开始时开启移动，显示提示
  (Variables|Default|SetIsGamePlaying true)
  (for _array_element (Variables|Default|GetPlayerList)
    (CallFunction|EventUpdateOnesGameInfo (Variables|/Game/Blueprint/GameController/PC_RobHat.PC_RobHat_C|GetPlayerGameInfo _array_element))
    (Default|EventUIInit _array_element)
    (bind _ascharacter_rob_hat (Utilities|Casting|CastToCharacter_RobHat (Pawn|GetControlledPawn _array_element)))
    (Pawn|Components|CharacterMovement|SetMovementMode (Variables|/Script/Engine.Character|GetCharacterMovement _ascharacter_rob_hat) "MOVE_Walking" 0)
    (Default|EventUIShowGameStart _array_element)
    (bind _returnvalue (Utilities|Time|SetTimerbyFunctionName 0 "Event_GamePlayCountDown" 1.0 true))))

(event Custom|Event_GamePlayCountDown
  ;[1 1 1] 游戏进行倒计时，结束后调用END
  (bind _output_get (Variables|Default|SetTimeCountDown (Variables|Default|GetTimeOfOnceGame)))
  (if (< _output_get 16)
    (CallFunction|EventUpdateAllCountDown))
  (if (> (Variables|Default|GetTimeOfOnceGame) 0)
    (Variables|Default|SetTimeOfOnceGame (- (Variables|Default|GetTimeOfOnceGame) 1))
    (else
      (Utilities|Time|ClearandInvalidateTimerbyHandle (stale Custom|Event_WhenGameStart _returnvalue))
      (CallFunction|EventwhenGamePlayEnd))))

(event EventBeginPlay
  ;[1 1 1] 进入Level后，游戏同步倒计时结束才允许移动
  (bind _returnvalue (Utilities|Time|SetTimerbyFunctionName 0 "Event_Timer_StartGame" 1.0 true)))

(event EventPostLogin
  (params (NewPlayer :type Player%20Controller%20Object%20Reference))
  ;[1 1 1] 玩家登录注册
  (Networking|SwitchHasAuthority
    (:Authority
      (bind _aspc_rob_hat (Utilities|Casting|CastToPC_RobHat NewPlayer))
      (bind _returnvalue (Utilities|Array|Add (Variables|Default|GetPlayerList) _aspc_rob_hat))
      (Utilities|Struct|SetmembersinRobHatPlayerInfoStruct (Variables|/Game/Blueprint/GameController/PC_RobHat.PC_RobHat_C|GetPlayerGameInfo _aspc_rob_hat) _returnvalue)
      (Default|EventAddSelftoGM _aspc_rob_hat _returnvalue)
      (CallFunction|EventInitSapwnPlayer _aspc_rob_hat))))

(fn ConstructionScript)