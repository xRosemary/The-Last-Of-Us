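; Player controller for the RobHat multiplayer shooter, handling HUD, player input, death and match-end screens.
; Input drives the possessed Character_RobHat: pickup, reload, timer-looped automatic fire, timeline FOV aiming.
; It registers player info with GM_RobHat, which handles KDA and respawns; RepNotifies refresh the HUD or push info back.
; On death it respawns the player after a delay, or shows game-over and destroys itself under GM_PlayWithAI.
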(event Custom|Event_ShowGameHUD
  ;[1 1 1] 初始化HUD
  (Viewport|RemoveAllWidgets)
  (bind _returnvalue (UserInterface|CreateWidget "/Game/Blueprint/UI/Game/RobHatHUD.RobHatHUD_C" self (.name (Variables|Default|GetPlayerGameInfo))))
  (bind _output_get (Variables|Default|SetRobHatHUD _returnvalue))
  (UserInterface|Viewport|AddtoViewport _output_get 0)
  (Variables|Default|SetbShowMouseCursor false)
  (Class|GameplayStatics|SetViewportMouseCaptureMode "CapturePermanently")
  (Class|WidgetBlueprintLibrary|SetFocustoGameViewport))

(event Custom|Event_PickUpSomeThing
  ;[1 1 1] 捡东西，由不同类型的东西来调用pawn的对应类型的捡东西函数
  (bind _ascharacter_rob_hat (Utilities|Casting|CastToCharacter_RobHat (Pawn|GetControlledPawn)))
  (Utilities|IsValid (Utilities|Array|Get(acopy) (Variables|/Game/Blueprint/Character_RobHat.Character_RobHat_C|GetPickUpList _ascharacter_rob_hat))
    (:Is%20Valid
      (Class|CanbePickUp|PickUp(Message) (Utilities|Array|Get(acopy) (Variables|/Game/Blueprint/Character_RobHat.Character_RobHat_C|GetPickUpList _ascharacter_rob_hat)) (Pawn|GetControlledPawn)))))

(event Custom|Event_UI_UpdatePlayersInfo
  (bind _robhathud (Variables|Default|GetRobHatHUD))
  ;[1 1 1] UI更新
  (Utilities|IsValid _robhathud
    (:Is%20Valid
      (Default|EventUpdatePlayerInfo _robhathud (Variables|Default|GetAllPlayerGameInfo)))))

(event Custom|Event_UI_Init
  (bind _robhathud (Variables|Default|GetRobHatHUD))
  ;[1 1 1] UI更新
  (Utilities|IsValid _robhathud
    (:Is%20Valid
      (Default|EventInitHUD _robhathud (Variables|Default|GetAllPlayerGameInfo)))))

(event Custom|Event_EntryFireState
  ;[1 1 1] 控制长按开火CD
  (bind _ascharacter_rob_hat (Utilities|Casting|CastToCharacter_RobHat (Pawn|GetControlledPawn)))
  (Utilities|IsValid (Variables|/Game/Blueprint/Character_RobHat.Character_RobHat_C|GetNowUseGun _ascharacter_rob_hat)
    (:Is%20Valid
      (bind _returnvalue (Utilities|Time|SetTimerbyFunctionName 0 "Event_ServeFire" (Variables|/Game/Blueprint/InterfaceAndBase/BaseGun.BaseGun_C|GetFireCD (Variables|/Game/Blueprint/Character_RobHat.Character_RobHat_C|GetNowUseGun _ascharacter_rob_hat)) true (- 0.0 (Variables|/Game/Blueprint/InterfaceAndBase/BaseGun.BaseGun_C|GetFireCD (Variables|/Game/Blueprint/Character_RobHat.Character_RobHat_C|GetNowUseGun _ascharacter_rob_hat))))))))

(event Custom|Event_CallServerUpdateMyInfo
  ;[1 1 1] 叫GM更新Infolist中的该PC的数据
  (bind _asgm_rob_hat (Utilities|Casting|CastToGM_RobHat (Game|GetGameMode)))
  (Default|EventUpdateOnesGameInfo _asgm_rob_hat (Variables|Default|GetPlayerGameInfo)))

(event Custom|Event_QuitFireState
  ;[1 1 1] 控制长按开火CD
  (Utilities|Time|ClearandInvalidateTimerbyHandle (stale Custom|Event_EntryFireState _returnvalue)))

(event Custom|Event_WhenPawnDied
  (params (Killer :type Actor%20Object%20Reference))
  ;[1 1 1] 当pawn死亡时
  (Utilities|Casting|CastToGM_PlayWithAI (Game|GetGameMode)
    (:then
      ;;[1 1 1] 单机死亡
      (CallFunction|EventDisableInput)
      (CallFunction|EventUIShowWaitReborn)
      (Utilities|FlowControl|Delay 2.0)
      (bind _returnvalue (UserInterface|CreateWidget "/Game/Blueprint/UI/Game/UI_GameOver.UI_GameOver_C" self))
      (UserInterface|Viewport|AddtoViewport _returnvalue 0)
      (Variables|Default|SetbShowMouseCursor true)
      (Actor|DestroyActor))
    (:CastFailed
      (CallFunction|EventUIKDADied Killer)
      (CallFunction|EventDisableInput)
      (CallFunction|EventUIShowWaitReborn)
      (Utilities|FlowControl|Delay (Variables|Default|GetRebornTime))
      (CallFunction|EventUIHideWaitReborn)
      (CallFunction|EventReborn)
      (Utilities|FlowControl|Delay 0.5)
      (CallFunction|EventUIUpdateHealth))))

(event Custom|Event_EntryAimMode
  ;[1 1 1] 设置开镜
  (bind _ascharacter_rob_hat (Utilities|Casting|CastToCharacter_RobHat (Pawn|GetControlledPawn)))
  (Variables|/Game/Blueprint/Character_RobHat.Character_RobHat_C|SetbIsAimMode _ascharacter_rob_hat true))

(event Custom|Event_QuitAimMode
  ;[1 1 1] 设置开镜
  (bind _ascharacter_rob_hat (Utilities|Casting|CastToCharacter_RobHat (Pawn|GetControlledPawn)))
  (Variables|/Game/Blueprint/Character_RobHat.Character_RobHat_C|SetbIsAimMode _ascharacter_rob_hat false))

(event Custom|Event_UI_ShowBeDamagedEffect
  ;[1 1 1] 命中反馈和受击反馈
  (if (Pawn|IsLocalPlayerController)
    (Default|EventShowbeDamaged (Variables|Default|GetRobHatHUD))))

(event Custom|Event_UI_ShowHitPawnEffect
  ;[1 1 1] 命中反馈和受击反馈
  (if (Pawn|IsLocalPlayerController)
    (Default|EventShowHitReaction (Variables|Default|GetRobHatHUD))))

(event Custom|Event_PCInit
  ;[1 1 1] 初始化HUD等，delay是等大家登陆完成
  (CallFunction|EventShowGameHUD)
  (Utilities|FlowControl|Delay 2.0)
  (CallFunction|EventUIInit))

(event Custom|Event_UI_ShowWaitReborn
  ;[1 1 1] 等待复活UI
  (Default|EventShowWaitReborn (Variables|Default|GetRobHatHUD)))

(event Custom|Event_UI_KDA_Died
  (params (Killer :type Actor%20Object%20Reference))
  ;[1 1 1] 修改KDA
  (bind _ascharacter_rob_hat (Utilities|Casting|CastToCharacter_RobHat Killer))
  (bind _aspc_rob_hat (Utilities|Casting|CastToPC_RobHat (Pawn|GetController _ascharacter_rob_hat)))
  (bind _asgm_rob_hat (Utilities|Casting|CastToGM_RobHat (Game|GetGameMode)))
  (Default|EventUpdateKDA _asgm_rob_hat _aspc_rob_hat self)
  (CallFunction|EventCallServerUpdateMyInfo _aspc_rob_hat))

(event Custom|Event_UI_HideWaitReborn
  ;[1 1 1] 等待复活UI
  (Default|EventHideWaitReborn (Variables|Default|GetRobHatHUD)))

(event Custom|Event_Reborn
  ;[1 1 1] 当pawn死亡时
  (bind _asgm_rob_hat (Utilities|Casting|CastToGM_RobHat (Game|GetGameMode)))
  (Default|EventRebornPawn _asgm_rob_hat self)
  (CallFunction|EventEnableInput))

(event Custom|Event_GetSertveCountDown
  (params (CountDown :type Integer))
  ;[1 1 1] 更新倒计时
  (bind _output_get (Variables|Default|SetCountDown CountDown))
  (CallFunction|EventUIUpdateCountDown _output_get))

(event Custom|Event_UI_UpdateCountDown
  (params (CountDown :type Integer))
  ;[1 1 1] 更新倒计时
  (Default|EventUpdateCountDown (Variables|Default|GetRobHatHUD) CountDown))

(event Custom|Event_UI_ShowGameStart
  ;[1 1 1] 显示游戏开始
  (Default|EventShowGameStart (Variables|Default|GetRobHatHUD)))

(event Custom|Event_WhenGameEnd
  (params (Winner :type Integer))
  ;[1 1 1] 游戏结束
  (CallFunction|EventUIShowGameEnd Winner)
  (Input|DisableInput (Pawn|GetControlledPawn) self))

(event Custom|Event_UI_ShowGameEnd
  (params (winner :type Integer))
  ;[1 1 1] 游戏结束UI
  (bind _returnvalue (UserInterface|CreateWidget "/Game/Blueprint/UI/Game/UI_GameEnd.UI_GameEnd_C" self))
  (UserInterface|Viewport|AddtoViewport _returnvalue 0)
  (Default|EventUpdatePlayerInfo _returnvalue (Variables|Default|GetAllPlayerGameInfo) winner))

(event Custom|Event_UI_UpdateHealthByValue
  (params (Health :type Integer))
  ;[1 1 1] UI更新
  (Default|EventUpdateHealthbyValue (Variables|Default|GetRobHatHUD) Health))

(event Custom|Event_DisableInput
  ;[1 1 1] 禁止输入
  (bind _as角色 (Utilities|Casting|CastToCharacter (Pawn|GetControlledPawn)))
  (Pawn|Components|CharacterMovement|DisableMovement (Variables|/Script/Engine.Character|GetCharacterMovement _as角色))
  (Input|DisableInput _as角色 0)
  (Input|DisableInput 0))

(event Custom|Event_EnableInput
  ;[1 1 1] 启用输入
  (Input|EnableInput 0))

(event Custom|Event_AddGameInfoToServer
  (params (GameInfo :type Rob%20Hat%20Player%20Info%20Struct%20Structure))
  ;[1 1 1] GameMode调用，将个人信息初始化的同时传给GM
  ;;[1 1 1] 信息添加到服务器
  (Variables|Default|SetPlayerGameInfo GameInfo)
  (bind _asgm_rob_hat (Utilities|Casting|CastToGM_RobHat (Game|GetGameMode)))
  (Default|EventAddPlayerGameInfo _asgm_rob_hat GameInfo))

(event Custom|Event_AddSelfToGM
  (params (PlayerNumber :type Integer))
  ;[1 1 1] GameMode调用，将个人信息初始化的同时传给GM
  (bind _asgame_instance_main (Utilities|Casting|CastToGameInstance_Main (Game|GetGameInstance)))
  (bind _output_get (Variables|Default|SetPlayerGameInfo (Utilities|Struct|MakeRobHatPlayerInfoStruct (.name (Variables|/Game/Blueprint/GameController/GameInstance_Main.GameInstance_Main_C|GetPlayerInfo _asgame_instance_main)) PlayerNumber 0 0 0)))
  (CallFunction|EventAddGameInfotoServer _output_get))

(event Custom|Event_ServeFire
  ;[1 1 1] 开火
  (bind _ascharacter_rob_hat (Utilities|Casting|CastToCharacter_RobHat (Pawn|GetControlledPawn)))
  (Default|EventUpdateFireVector _ascharacter_rob_hat (Math|Vector|GetForwardVector (Variables|/Game/Blueprint/Character_RobHat.Character_RobHat_C|GetFollowCamera _ascharacter_rob_hat)))
  (Default|EventOpenFire _ascharacter_rob_hat)
  (CallFunction|EventUIUpdateWeapon))

(event Custom|Event_ReloadBullet
  (bind _returnvalue (Pawn|GetControlledPawn))
  ;[1 1 1] 换弹
  (Utilities|IsValid _returnvalue
    (:Is%20Valid
      (bind _ascharacter_rob_hat (Utilities|Casting|CastToCharacter_RobHat _returnvalue))
      (Default|EventReloadBullet _ascharacter_rob_hat))))

(event Custom|Event_UI_UpdateWeapon
  (bind _robhathud (Variables|Default|GetRobHatHUD))
  ;[1 1 1] UI更新
  (Utilities|IsValid _robhathud
    (:Is%20Valid
      (Default|EventUpdateAmor _robhathud))))

(event Custom|Event_UI_UpdateHealth
  (bind _robhathud (Variables|Default|GetRobHatHUD))
  ;[1 1 1] UI更新
  (Utilities|IsValid _robhathud
    (:Is%20Valid
      (Default|EventUpdateHealth _robhathud))))

(event EventBeginPlay
  ;[1 1 1] 初始化HUD等，delay是等大家登陆完成
  (CallFunction|EventPCInit))

(event Input|ActionEvents|InputActionWhenESC
  (params (Key :type Key%20Structure))
  ;[1 1 1] 退出游戏
  (:Pressed
    (Utilities|FlowControl|FlipFlop
      (:A
        (Game|SetGamePaused true)
        (bind _returnvalue (UserInterface|CreateWidget "/Game/Blueprint/UI/Game/UI_PauseSEC.UI_PauseSEC_C" self))
        (UserInterface|Viewport|AddtoViewport _returnvalue 0)
        (Variables|Default|SetbShowMouseCursor true))
      (:B
        (Widget|RemovefromParent _returnvalue)
        (Variables|Default|SetbShowMouseCursor false)))))

(event Input|ActionEvents|InputActionLeftClick
  (params (Key :type Key%20Structure))
  ;[1 1 1] 开火
  (:Pressed
    (CallFunction|EventEntryFireState))
  (:Released
    (CallFunction|EventQuitFireState)))

(event Input|ActionEvents|InputActionPickUp
  (params (Key :type Key%20Structure))
  ;[1 1 1] 捡东西，由不同类型的东西来调用pawn的对应类型的捡东西函数
  (:Pressed
    (CallFunction|EventPickUpSomeThing)
    (Networking|SwitchHasAuthority
      (:Authority
        (CallFunction|EventUIUpdateWeapon))
      (:Remote
        (Utilities|FlowControl|Delay 0.2)
        (CallFunction|EventUIUpdateWeapon)))))

(event Input|ActionEvents|InputActionRightClick
  (params (Key :type Key%20Structure))
  ;[1 1 1] 设置开镜
  (:Pressed
    (bind _ascharacter_rob_hat (Utilities|Casting|CastToCharacter_RobHat (Pawn|GetControlledPawn)))
    (Utilities|IsValid (Variables|/Game/Blueprint/Character_RobHat.Character_RobHat_C|GetNowUseGun _ascharacter_rob_hat)
      (:Is%20Valid
        (CallFunction|EventEntryAimMode)
        (bind _fieldofview (Timeline|ViewFieldTimeLine Play)
          (:Update
            (Variables|/Script/Engine.CameraComponent|SetFieldOfView (Variables|/Game/Blueprint/Character_RobHat.Character_RobHat_C|GetFollowCamera _ascharacter_rob_hat) _fieldofview))))))
  (:Released
    (bind _ascharacter_rob_hat_2 (Utilities|Casting|CastToCharacter_RobHat (Pawn|GetControlledPawn)))
    (Utilities|IsValid (Variables|/Game/Blueprint/Character_RobHat.Character_RobHat_C|GetNowUseGun _ascharacter_rob_hat_2)
      (:Is%20Valid
        (CallFunction|EventQuitAimMode)
        (Timeline|ViewFieldTimeLine Reverse)))))

(event Input|ActionEvents|InputActionReBullet
  (params (Key :type Key%20Structure))
  ;[1 1 1] 换弹
  (:Pressed
    (CallFunction|EventReloadBullet)))

(event Input|ActionEvents|InputActionTabHUD
  (params (Key :type Key%20Structure))
  ;[1 1 1] 切换提示
  (:Pressed
    (Default|EventToggleHint (Variables|Default|GetRobHatHUD))))

(event Input|ActionEvents|InputActionTest
  (params (Key :type Key%20Structure))
  ;[1 1 1] 退出游戏
)

(fn ConstructionScript
  (CallFunction|EventUIUpdatePlayersInfo))

(fn OnRepAllPlayerGameInfo
  (CallFunction|EventUIUpdatePlayersInfo))

(fn OnRepPlayerGameInfo
  (CallFunction|EventCallServerUpdateMyInfo))